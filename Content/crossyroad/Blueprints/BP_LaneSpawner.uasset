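; Lane spawner for a Crossy Road-style game that builds a chain of random lanes, starting at BeginPlay.
; Each new lane spawns at the newest lane's SpawnPoint, from grass, road or water variants; the BP_Grass2 case lies outside the random range.
; Once the list reaches its cap, each spawn clears the oldest lane's Expiring flag, decrements TimeToLive on expiring lanes and destroys depleted ones.
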(event `self.ReceiveBeginPlay`
  (`self.SpawnInitialLanes`))

(fn `RandomLane`
  (params (SpawnLocation :type "Vector Structure"))
  (returns (ReturnValue :type "/Game/crossyroad/Blueprints/BP_Lane Object Reference") (ReturnValue1 :type "/Game/crossyroad/Blueprints/BP_Grass1 Object Reference"))
  (switch `int` (`KismetMathLibrary.RandomIntegerInRange` 0 3)
    (:`0`
      (bind _returnvalue (`|SpawnActorFromClass` "/Game/crossyroad/Blueprints/BP_Grass1.BP_Grass1_C" (`KismetMathLibrary.MakeTransform` SpawnLocation (struct) (100.0 100.0 100.0)) "Undefined" "OverrideRootScale" null null))
      (return null _returnvalue))
    (:`1`
      (`|SpawnActorFromClass` "/Game/crossyroad/Blueprints/BP_Road.BP_Road_C" (`KismetMathLibrary.MakeTransform` SpawnLocation (struct) (100.0 100.0 100.0)) "Undefined" "OverrideRootScale" null null))
    (:`2`
      (`|SpawnActorFromClass` "/Game/crossyroad/Blueprints/BP_Water.BP_Water_C" (`KismetMathLibrary.MakeTransform` SpawnLocation (struct) (100.0 100.0 100.0)) "Undefined" "OverrideRootScale" null null))
    (:`3`
      (`|SpawnActorFromClass` "/Game/crossyroad/Blueprints/BP_Tracks.BP_Tracks_C" (`KismetMathLibrary.MakeTransform` SpawnLocation (struct) (100.0 100.0 100.0)) "Undefined" "OverrideRootScale" null null))
    (:`4`
      (`|SpawnActorFromClass` "/Game/crossyroad/Blueprints/BP_Grass2.BP_Grass2_C" (`KismetMathLibrary.MakeTransform` SpawnLocation (struct) (100.0 100.0 100.0)) "Undefined" "OverrideRootScale" null null))))

(fn `SpawnInitialLanes`
  (for _ (range 5)
    (`/Engine/EditorBlueprintResources/StandardMacros.IsValid` (`self.NewestLane`)
      (:`Is Valid`
        (`self.SpawnLaneAtSpawnPoint`))
      (:`Is Not Valid`
        (`self.SpawnLane` (400.0 0.0 20.0))))))

(fn `SpawnLane`
  (params (SpawnLocation :type "Vector Structure"))
  (bind _returnvalue (`self.RandomLane` SpawnLocation))
  (bind _output_get (set `self.NewestLane` _returnvalue))
  (set `/Game/crossyroad/Blueprints/BP_Lane.LaneSpawner` self _output_get)
  (`KismetArrayLibrary.Array_Add` (`self.Lanes`) _output_get)
  (if (>= (`KismetArrayLibrary.Array_Length` (`self.Lanes`)) 25)
    (set `/Game/crossyroad/Blueprints/BP_Lane.Expiring` false (`|GetArrayItem` (`self.Lanes`)))
    (`self.UpdateLaneCounter`)))

(fn `SpawnLaneAtSpawnPoint`
  (`self.SpawnLane` (`SceneComponent.K2_GetComponentLocation` (`/Game/crossyroad/Blueprints/BP_Lane.SpawnPoint` (`self.NewestLane`)))))

(fn `UpdateLaneCounter`
  (bind _lanes (`self.Lanes`))
  (for _array_element (`self.Lanes`)
    (if (`/Game/crossyroad/Blueprints/BP_Lane.Expiring` _array_element)
      (set `/Game/crossyroad/Blueprints/BP_Lane.TimeToLive` (- (`/Game/crossyroad/Blueprints/BP_Lane.TimeToLive` _array_element) 1) _array_element)))
  (bind (_arrayindex _arrayelement) (`/Engine/EditorBlueprintResources/StandardMacros.ReverseForEachLoop` _lanes)
    (:`LoopBody`
      (if (<= (`/Game/crossyroad/Blueprints/BP_Lane.TimeToLive` _arrayelement) 0)
        (`self.K2_DestroyActor` _arrayelement)
        (`KismetArrayLibrary.Array_Remove` _lanes _arrayindex)))))

(fn `UserConstructionScript`)