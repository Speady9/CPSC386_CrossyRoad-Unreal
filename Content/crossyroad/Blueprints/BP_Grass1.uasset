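; BP_Grass1 is a grass tile, apparently for a Crossy Road-style game, that randomizes its obstacle dressing in the Construction Script.
; It shuffles eight obstacle marker components and runs an empty loop up to a random count.
; After the loop, one static mesh component is added at the location of the indexed marker.
; A random three-way switch sets its mesh, though no mesh assets are shown, and the event graph is unused.
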(fn `UserConstructionScript`
  (bind _array (`|MakeArray` (`self.Obstacle0`) (`self.Obstacle1`) (`self.Obstacle2`) (`self.Obstacle3`) (`self.Obstacle4`) (`self.Obstacle5`) (`self.Obstacle6`) (`self.Obstacle7`)))
  (`KismetArrayLibrary.Array_Shuffle` _array)
  (for _index (range (+ (`KismetMathLibrary.RandomInteger` (`KismetArrayLibrary.Array_Length` _array)) 1))
    _)
  (bind _returnvalue (`AddComponent|NODE_AddStaticMeshComponent-2` :`RelativeTransform` (`KismetMathLibrary.MakeTransform` (`SceneComponent.RelativeLocation` (`|GetArrayItem` _array _index)))))
  (switch `int` (`KismetMathLibrary.RandomInteger` 3)
    (:`0`
      (`StaticMeshComponent.SetStaticMesh` _returnvalue null))
    (:`1`
      (`StaticMeshComponent.SetStaticMesh` _returnvalue null))
    (:`2`
      (`StaticMeshComponent.SetStaticMesh` _returnvalue null))))