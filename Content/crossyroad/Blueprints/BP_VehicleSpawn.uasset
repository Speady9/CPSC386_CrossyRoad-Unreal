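; BP_VehicleSpawn is a spawner actor that places randomized BP_Vehicle actors in the crossyroad game.
; On BeginPlay it destroys every BP_Vehicle in the world, then runs a single-pass loop that spawns at the newest vehicle's location if valid, otherwise at its own root.
; Each spawned vehicle is stored as NewestVehicle, receives a back-reference to the spawner and randomizes itself.
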(event `self.ReceiveBeginPlay`
  (`self.SpawnInitialVehicle`))

(fn `SpawnInitialVehicle`
  (`|ExecutionSequence`
    (:`then_0`
      (bind _outactors (`GameplayStatics.GetAllActorsOfClass` "/Game/crossyroad/Blueprints/BP_Vehicle.BP_Vehicle_C"))
      (for _array_element _outactors
        (`self.K2_DestroyActor` _array_element)))
    (:`then_1`
      (for _ (range 1)
        (`/Engine/EditorBlueprintResources/StandardMacros.IsValid` (`self.Newest Vehicle`)
          (:`Is Valid`
            (`self.SpawnVehicleAtSpawnPoint`))
          (:`Is Not Valid`
            (`self.SpawnVehicle` (`SceneComponent.K2_GetComponentLocation` (`self.DefaultSceneRoot`)))))))))

(fn `SpawnVehicle`
  (params (SpawnLocation :type "Vector Structure"))
  (bind _returnvalue (`|SpawnActorFromClass` "/Game/crossyroad/Blueprints/BP_Vehicle.BP_Vehicle_C" (`KismetMathLibrary.MakeTransform` SpawnLocation) "Undefined" "OverrideRootScale" null null))
  (bind _output_get (set `self.Newest Vehicle` _returnvalue))
  (set `/Game/crossyroad/Blueprints/BP_Vehicle.VehicleSpawner` self _output_get)
  (`/Game/crossyroad/Blueprints/BP_Vehicle.RandomizeVehicle` _output_get))

(fn `SpawnVehicleAtSpawnPoint`
  (`self.SpawnVehicle` (`SceneComponent.K2_GetComponentLocation` (`Actor.RootComponent` (`self.Newest Vehicle`)))))

(fn `UserConstructionScript`)