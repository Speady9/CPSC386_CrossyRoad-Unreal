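; BP_Chicken is the player-controlled chicken in the crossyroad game, moved forward along world negative Y.
; Tick re-enables input every frame and feeds the Move variable into AddMovementInput as its scale.
; Pressing W or the Jump action sets Move to Forwards, then to Stop after a one-second delay.
; Releasing W also re-enables input and sets Move to Stop immediately.
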(event `self.ReceiveTick`
  (params (DeltaSeconds :type "Float (single-precision)"))
  (`self.EnableInput` null)
  (`self.AddMovementInput` (0.0 -1.0 0.0) (`self.Move`)))

(event `InputAction|ActionInput Jump`
  (params (Key :type "Key Structure"))
  (:`Pressed`
    (set `self.Move` (`self.Forwards`) :!label _label)
    (`KismetSystemLibrary.Delay` 1.0)
    (set `self.Move` (`self.Stop`) :!label _label_2)))

(event `Key|W`
  (params (Key :type "Key Structure"))
  (:`Pressed`
    (goto _label))
  (:`Released`
    (`self.EnableInput` null)
    (goto _label_2)))

(fn `UserConstructionScript`)