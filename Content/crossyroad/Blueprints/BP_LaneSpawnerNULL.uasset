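; BP_LaneSpawnerNULL is a spawner actor that lays out the initial run of BP_LaneNULL lanes for the crossyroad game.
; On BeginPlay it loops to spawn lanes, placing the first at the player pawn's location and each later one at a SpawnPoint's world location.
; Each spawn is stored as NewestLane, whose validity selects the position, and a LaneSpawner reference is set to this actor.
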(event `self.ReceiveBeginPlay`
  (`self.SpawnInitialLanes`))

(fn `SpawnInitialLanes`
  (for _ (range 11)
    (`/Engine/EditorBlueprintResources/StandardMacros.IsValid` (`self.NewestLane`)
      (:`Is Valid`
        (`self.SpawnLaneAtSpawnPoint`))
      (:`Is Not Valid`
        (`self.SpawnLane` (`self.K2_GetActorLocation` (`GameplayStatics.GetPlayerPawn` 0)))))))

(fn `SpawnLane`
  (params (SpawnLocation :type "Vector Structure"))
  (bind _returnvalue (`|SpawnActorFromClass` "/Game/crossyroad/Blueprints/BP_LaneNULL.BP_LaneNULL_C" (`KismetMathLibrary.MakeTransform` SpawnLocation) "Undefined" "OverrideRootScale" null null))
  (set `self.NewestLane` _returnvalue)
  (set `self.LaneSpawner` self))

(fn `SpawnLaneAtSpawnPoint`
  (`self.SpawnLane` (`SceneComponent.K2_GetComponentLocation` (`self.SpawnPoint`))))

(fn `UserConstructionScript`)