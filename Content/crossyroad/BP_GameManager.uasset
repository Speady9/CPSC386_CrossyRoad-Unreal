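; Game manager pawn for a Crossy Road-style game, serving as the auto-scrolling camera and tracking score, coins and high score.
; Tick moves it along +X until the player is hit, and CheckPlayer spawns a single eagle once the player's position fails screen projection.
; IncrementScore and IncrementCoins update the score widget created on BeginPlay.
; The high score loads from a save slot in the construction script and saves on EndPlay.
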(event `self.ReceiveBeginPlay`
  (bind _returnvalue (`|CreateWidget` null))
  (`UserWidget.AddToViewport` _returnvalue 0)
  (set `/Game/crossyroad/BP_GameManager.GameManager` self _returnvalue)
  (set `self.ScoreWidget` null _returnvalue)
  (set `self.bFindCameraComponentWhenViewTarget` true)
  (`PlayerController.SetViewTargetWithBlend` (`GameplayStatics.GetPlayerController` 0) self 0.0 "VTBlend_Linear" 0.0 false)
  (bind _outactors (`GameplayStatics.GetAllActorsOfClass` null))
  (set `self.Player` null null)
  (`self.UpdateTopScore` (`.ScoreWidget` (`self.ScoreWidget`))))

(event `self.ReceiveTick`
  (params (DeltaSeconds :type "Float (single-precision)"))
  (if (not (`/Game/crossyroad/BP_GameManager.Hit` (`.Player` (`self.Player`))))
    (`self.AddMovementInput` (1.0 0.0 0.0) 100.0)
    (bind _returnvalue (`self.ConsumeMovementInputVector`))
    (`self.K2_AddActorLocalOffset` (* _returnvalue DeltaSeconds) true)
    (`self.CheckPlayer`)))

(event `self.ReceiveEndPlay`
  (params (EndPlayReason :type "EEndPlayReason Enum" :default "Destroyed"))
  (bind (_savegameinstance _savegameinstance_2) (`self.SaveGameInstance`))
  (set `/Game/crossyroad/BP_GameManager.HighScore` (`self.CurrentHighScore`) _savegameinstance_2)
  (`GameplayStatics.SaveGameToSlot` _savegameinstance_2 (`/Game/crossyroad/BP_GameManager.SaveFileID` _savegameinstance_2))
  (`KismetSystemLibrary.PrintString` "Saved game data"))

(fn `CheckPlayer`
  (bind (_returnvalue_x _returnvalue_y _returnvalue_z) (`KismetMathLibrary.BreakVector` (`self.K2_GetActorLocation` (`.Player` (`self.Player`)))))
  (if (`.ReturnValue` (`GameplayStatics.ProjectWorldToScreen` (`GameplayStatics.GetPlayerController` 0) (`self.K2_GetActorLocation` (`.Player` (`self.Player`))) true))
    _
    (elif (not (`self.EagleSent`))
      (bind _returnvalue (`|SpawnActorFromClass` null (`KismetMathLibrary.MakeTransform` (`KismetMathLibrary.MakeVector` (+ _returnvalue_x 800.0) _returnvalue_y (+ _returnvalue_z 100.0))) "Undefined" "OverrideRootScale" null null))
      (set `/Game/crossyroad/BP_GameManager.Player` (`.Player` (`self.Player`)) _returnvalue)
      (set `self.EagleSent` true))))

(fn `IncrementCoins`
  (`/Engine/EditorBlueprintResources/StandardMacros.IncrementInt` (`self.CoinsCollected`)
    (:`  `
      (`self.UpdateCoinCounter` (`.ScoreWidget` (`self.ScoreWidget`))))))

(fn `IncrementScore`
  (bind _output_get (set `self.Score` (+ (`self.Score`) 1)))
  (`self.UpdateScoreCounter` (`.ScoreWidget` (`self.ScoreWidget`)))
  (if (> _output_get (`self.CurrentHighScore`))
    (set `self.CurrentHighScore` (`self.Score`))
    (`self.UpdateTopScore` (`.ScoreWidget` (`self.ScoreWidget`)))))

(fn `UserConstructionScript`
  (bind _returnvalue (`GameplayStatics.CreateSaveGameObject` null))
  (bind (_output_get _output_get_2) (set `self.SaveGameInstance` null _returnvalue))
  (bind _returnvalue_2 (`GameplayStatics.LoadGameFromSlot` (`/Game/crossyroad/BP_GameManager.SaveFileID` _output_get_2)))
  (bind _asbp_save_high_score (cast `` _returnvalue_2))
  (bind (_output_get_3 _output_get_4) (set `self.SaveGameInstance` null _asbp_save_high_score))
  (set `self.CurrentHighScore` (`/Game/crossyroad/BP_GameManager.HighScore` _output_get_4))
  (`KismetSystemLibrary.PrintString` "Loaded game data"))